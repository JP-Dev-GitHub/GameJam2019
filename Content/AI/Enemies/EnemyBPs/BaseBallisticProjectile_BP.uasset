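; Base Blueprint for a ballistic projectile under enemy AI, launched at a configurable speed with a maximum lifespan set in the construction script.
; The first hit or box overlap with an actor outside the ignore list triggers HitEvent.
; HitEvent hides the AIM9 component, stops the trail, spawns particles and plays sound at world origin, leaving cleanup to the lifespan.
; A looping timer records LastLocation, which is unread here.
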(event OnComponentBeginOverlap(BoxCollider)
  (params (OverlappedComponent :type Primitive%20Component%20Object%20Reference) (OtherActor :type Actor%20Object%20Reference) (OtherComp :type Primitive%20Component%20Object%20Reference) (OtherBodyIndex :type Integer) (bFromSweep :type Boolean) (SweepResult :type Hit%20Result%20Structure%20%28by%20ref%29))
  (if (Math|Boolean|ANDBoolean (Variables|Default|GetAlive?) (== (Utilities|Array|FindItem (Variables|Default|GetIgnoreActors) OtherActor) -1) (!= OtherActor self))
    (Variables|Default|SetAlive? false)
    (Variables|Default|SetHitParticleTransform (Math|Transform|MakeTransform (Transformation|GetActorLocation) "0, 0, 0" "0.500000,0.500000,0.500000"))
    (CallFunction|HitEvent)))

(event Custom|HitEvent
  (bind _hitparticletransform (Variables|Default|GetHitParticleTransform))
  (Variables|Default|SetAlive? false)
  (Rendering|SetVisibility (Variables|Default|GetAIM-9) false false)
  (Components|Activation|Deactivate (Variables|Default|GetTrail))
  (Effects|SpawnEmitteratLocation (Variables|Default|GetHitParticle) (.location _hitparticletransform) (.rotation _hitparticletransform) (.scale _hitparticletransform))
  (Audio|PlaySoundatLocation (Variables|Default|GetHitSound) "0, 0, 0" "0, 0, 0" 1.0 1.0 0.0 0 0 0))

(event Custom|UpdateLocation
  (Variables|Default|SetLastLocation (Transformation|GetActorLocation)))

(event EventBeginPlay
  (Utilities|Time|SetTimerbyFunctionName 0 "UpdateLocation" 0.15 true)
  (Variables|Default|SetLastLocation (Transformation|GetActorLocation)))

(event Collision|EventHit
  (params (MyComp :type Primitive%20Component%20Object%20Reference) (Other :type Actor%20Object%20Reference) (OtherComp :type Primitive%20Component%20Object%20Reference) (bSelfMoved :type Boolean) (HitLocation :type Vector :default "0, 0, 0") (HitNormal :type Vector :default "0, 0, 0") (NormalImpulse :type Vector :default "0, 0, 0") (Hit :type Hit%20Result%20Structure%20%28by%20ref%29))
  (if (Math|Boolean|ANDBoolean (Variables|Default|GetAlive?) (== (Utilities|Array|FindItem (Variables|Default|GetIgnoreActors) Other) -1) (!= Other self))
    (Variables|Default|SetAlive? false)
    (Variables|Default|SetHitParticleTransform (Math|Transform|MakeTransform (Transformation|GetActorLocation) "0, 0, 0" "0.500000,0.500000,0.500000"))
    (CallFunction|HitEvent)))

(fn ConstructionScript
  (Variables|/Script/Engine.ProjectileMovementComponent|SetInitialSpeed (Variables|Default|GetProjectileMovement) (Variables|Default|GetLaunchSpeed))
  (Actor|SetLifeSpan (Variables|Default|GetMaxLifetime)))