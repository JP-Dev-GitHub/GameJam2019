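; LaserBolt is a child projectile Blueprint for an enemy laser shot, setting its own launch speed, hit sound and impact particle in the construction script.
; On BeginPlay it tints the trail particle blue and enables query-only box collision after a short delay.
; On HitEvent it orients the scaled-down impact particle back toward LastLocation, against the direction of travel, then defers to the parent's hit logic.
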(event EventBeginPlay
  (|CallParentFunction)
  (Effects|Components|ParticleSystem|SetVectorParameter (Variables|Default|GetTrail) "Color" (Math|Conversions|ToVector(LinearColor) "(R=0.000000,G=34.999992,B=100.000000,A=1.000000)"))
  (Utilities|FlowControl|Delay 0.1)
  (Collision|SetCollisionEnabled (Variables|Default|GetBoxCollider) "QueryOnly"))

(event EventHitEvent
  (bind _returnvalue (Transformation|GetActorLocation))
  (Variables|Default|SetHitParticleTransform (Math|Transform|MakeTransform (Transformation|GetActorLocation) (Math|Rotator|FindLookatRotation _returnvalue (+ _returnvalue (* (Math|Vector|Normalize (- (Variables|Default|GetLastLocation) _returnvalue)) 3e+02))) "0.350000,0.350000,0.350000"))
  (|CallParentFunction))

(event Collision|EventHit
  (params (MyComp :type Primitive%20Component%20Object%20Reference) (Other :type Actor%20Object%20Reference) (OtherComp :type Primitive%20Component%20Object%20Reference) (bSelfMoved :type Boolean) (HitLocation :type Vector :default "0, 0, 0") (HitNormal :type Vector :default "0, 0, 0") (NormalImpulse :type Vector :default "0, 0, 0") (Hit :type Hit%20Result%20Structure%20%28by%20ref%29))
  (|CallParentFunction MyComp Other OtherComp bSelfMoved HitLocation HitNormal NormalImpulse Hit))

(fn ConstructionScript
  (Variables|Default|SetLaunchSpeed 5e+03)
  (Variables|Default|SetHitSound "/Engine/VREditor/Sounds/UI/Camera_Shutter.Camera_Shutter")
  (Variables|Default|SetHitParticle "/Game/Particles/P_LaserImpact.P_LaserImpact")
  (|CallParentFunction))