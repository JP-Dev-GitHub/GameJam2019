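; BC_SmallRocketLauncher is a weapon component that mounts a small rocket launcher on a modular low-poly robot.
; On BeginPlay it spawns the platform mesh at RootSocket on the robot body, then attaches the launcher mesh to that platform.
; Tick calls RotateGun to turn both platform and gun.
; It binds to the owner's fire activation, but the fire event is empty in this graph.
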(event Custom|fireEvent
  (params (value :type Boolean)))

(event EventBeginPlay
  (|CallParentFunction)
  (EventDispatchers|BindEventtoFireActivate (Variables|Default|GetOwnerRobot) (delegate Custom|fireEvent))
  (CallFunction|SpawnGunMesh "/Game/ModularLowPolyRobots/Meshes/RobotWeapons/SM_SmallRocketLauncherPlatform.SM_SmallRocketLauncherPlatform" (Variables|/Game/ModularLowPolyRobots/Blueprints/BP_mainRobotPart.BP_mainRobotPart_C|GetRobotBody (Variables|Default|GetOwnerRobot)) (Variables|Default|GetGunPlatform) (Variables|Default|GetRootSocket))
  (CallFunction|SpawnGunMesh "/Game/ModularLowPolyRobots/Meshes/RobotWeapons/SM_SmallRocketLauncher.SM_SmallRocketLauncher" (Variables|Default|GetGunPlatform) (Variables|Default|GetGunMesh) "Any"))

(event EventTick
  (params (DeltaSeconds :type Float%20%28single-precision%29))
  (CallFunction|RotateGun true true))