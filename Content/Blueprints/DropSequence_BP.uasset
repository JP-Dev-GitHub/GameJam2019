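; DropSequence_BP runs a scripted VR drop on BeginPlay, moving the player pawn from StartPoint to EndPoint and ending in a heavy landing.
; A timeline teleports the player along the path with looping controller rumble, then detaches them, intensifies rumble and plays an impact sound.
; A parallel delayed timeline shakes the head by offsetting VROrigin, then stops the rumble and plays a mechanical startup sound.
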(event Custom|Drop
  (bind _player (Variables|Default|GetPlayer))
  (bind _player_2 (Variables|Default|GetPlayer))
  (bind _player_3 (Variables|Default|GetPlayer))
  (bind _vrorigin (Variables|/Game/ArmIK/MechPawn.MechPawn_C|GetVROrigin _player))
  (bind _relativelocation (Variables|/Script/Engine.SceneComponent|GetRelativeLocation _vrorigin))
  ;[1 1 1] Ground Pound
  (Utilities|FlowControl|Sequence
    (:then_0
      (Default|RumbleController (Variables|Default|GetPlayer) "AnyHand" 0.5 true)
      (bind _alpha (Timeline|Drop_TL PlayFromStart)
        (:Update
          (Transformation|Teleport _player_3 (Math|Vector|Lerp(Vector) (Variables|Default|GetStartLocation) (Variables|Default|GetEndLocation) _alpha) (Transformation|GetActorRotation _player_3)))
        (:Finished
          (Transformation|Teleport _player_2 (Variables|Default|GetEndLocation) (Transformation|GetActorRotation _player_2))
          (Transformation|DetachFromActor (Variables|Default|GetPlayer) "KeepWorld" "KeepWorld" "KeepWorld")
          (Default|RumbleController (Variables|Default|GetPlayer) "AnyHand" 1.0 true)
          (Audio|PlaySound2D "/Game/Audio/GigaImpactLanding_Cue.GigaImpactLanding_Cue" 1.0 1.0 0.0 0 0))))
    (:then_1
      ;[1 1 1] Camera Shake
      (Utilities|FlowControl|Delay 1.75)
      (bind _alpha_2 (Timeline|Headshake_TL PlayFromStart)
        (:Update
          (Transformation|SetRelativeLocation _vrorigin (Math|Vector|MakeVector (Math|Float|Lerp 1e+01 -1e+01 _alpha_2) (.y _relativelocation) (.z _relativelocation)) false false))
        (:Finished
          (Default|StopRumbleLoop (Variables|Default|GetPlayer) "AnyHand")
          (Utilities|FlowControl|Delay 1.0)
          (Audio|PlaySound2D "/Game/Audio/Mechanical_Startup_Cue.Mechanical_Startup_Cue" 1.0 1.0 0.0 0 0))))))

(event EventBeginPlay
  (bind _playerpawn (CallFunction|GetPlayerPawn))
  (Variables|Default|SetStartLocation (Transformation|GetWorldLocation (Variables|Default|GetStartPoint)))
  (Variables|Default|SetEndLocation (Transformation|GetWorldLocation (Variables|Default|GetEndPoint)))
  (Utilities|IsValid _playerpawn
    (:Is%20Valid
      (bind _output_get (Variables|Default|SetPlayer _playerpawn))
      (EventDispatchers|BindEventtoDebugButtonPress _output_get (EventDispatchers|CreateEvent :!event Custom|Drop))
      (CallFunction|Drop))))

(fn ConstructionScript)