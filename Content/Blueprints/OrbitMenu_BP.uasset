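; OrbitMenu_BP is a world-space widget menu that floats in front of the player's camera while active.
; Each tick it computes a point along the camera's forward vector at a set distance and height offset, plus a rotation facing the camera, optionally yaw-only.
; It eases toward both with interpolated location and rotation.
; The construction script sizes the widget's draw area from an aspect ratio variable.
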(event EventBeginPlay
  (bind _playerpawn (CallFunction|GetPlayerPawn))
  (Utilities|IsValid _playerpawn
    (:Is%20Valid
      (Variables|Default|SetPlayerRef _playerpawn))))

(event EventTick
  (params (DeltaSeconds :type Float%20%28single-precision%29))
  (if (Variables|Default|GetActive?)
    (Utilities|IsValid (Variables|Default|GetPlayerRef)
      (:Is%20Valid
        (bind _targetlocation (CallFunction|FindOrbitLocation))
        (bind _targetrotation (CallFunction|FindOrbitRotation))
        (Transformation|SetActorLocationAndRotation (Math|Interpolation|VInterpTo (Transformation|GetActorLocation) _targetlocation DeltaSeconds (Variables|Default|GetMoveSpeed)) (Math|Interpolation|RInterpTo (Transformation|GetActorRotation) _targetrotation DeltaSeconds (Variables|Default|GetRotateSpeed)))))))

(fn ConstructionScript
  (Class|WidgetComponent|SetDrawSize (Variables|Default|GetWidget) (Variables|Default|GetAspectRatio)))

(fn FindOrbitLocation
  (bind _playerref (Variables|Default|GetPlayerRef))
  (bind _camera (Variables|/Game/ArmIK/MechPawn.MechPawn_C|GetCamera _playerref))
  (return (+ (+ (Transformation|GetWorldLocation _camera) (* (Math|Vector|GetForwardVector _camera) (Variables|Default|GetOrbitDistance))) (Math|Vector|MakeVector 0.0 0.0 (Variables|Default|GetHieghtOffset)))))

(fn FindOrbitRotation
  (bind _returnvalue (Transformation|GetActorLocation))
  (bind _playerref (Variables|Default|GetPlayerRef))
  (bind _camera (Variables|/Game/ArmIK/MechPawn.MechPawn_C|GetCamera _playerref))
  (bind _returnvalue_2 (Transformation|GetWorldLocation _camera))
  (bind _returnvalue_3 (Math|Rotator|FindLookatRotation _returnvalue _returnvalue_2))
  (if (Variables|Default|GetOnlyUseZ?)
    (return (Math|Rotator|MakeRotator 0.0 0.0 (.Yaw (Math|Rotator|BreakRotator _returnvalue_3))))
    (else
      (return _returnvalue_3))))