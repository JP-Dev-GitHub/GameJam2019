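; BuildingTool procedurally fills a city layout's lots with randomized buildings and props in its Construction Script.
; Children of the Lots component supply positions, stored with random quarter-turn rotations, though a roll of 4 matches no case and drops the lot.
; A weighted roll, favoring apartment child actors, otherwise picks static-mesh special buildings, empty lots, car grids or parks.
; The EventGraph holds only unreachable, deprecated chunk-based building code.
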(event Collision|EventActorBeginOverlap
  (params (OtherActor :type Actor%20Object%20Reference))
  ;[1 1 1] Deprecato
)

(event EventBeginPlay)

(fn ConstructionScript
  ;[0 0 0] Get & Save Lot Locations
  (for _array_element (Components|GetChildrenComponents (Variables|Default|GetLots) false)
    (switch int (Math|Random|RandomIntegerinRange 1 4)
      (:0
        (LocalVariables|SetRandomRotation "0,0.000000, 0"))
      (:1
        (LocalVariables|SetRandomRotation "0,90.000000, 0"))
      (:2
        (LocalVariables|SetRandomRotation "0,180.000000, 0"))
      (:3
        (LocalVariables|SetRandomRotation "0,270.000000, 0")))
    (Utilities|Array|Add (Variables|Default|GetLotTransforms) (Math|Transform|MakeTransform (Variables|/Script/Engine.SceneComponent|GetRelativeLocation _array_element) (LocalVariables|GetRandomRotation) (Variables|Default|GetBuildingScale))))
  (for _array_element_2 (Variables|Default|GetLotTransforms)
    (bind _lotcategory (CallFunction|RandomizeLotType))
    (switch Utilities|FlowControl|Switch|SwitchonLotCategory _lotcategory
      (:NewEnumerator0
        (CallFunction|GenerateApartment _array_element_2))
      (:NewEnumerator1
        (CallFunction|GenerateSpecialBuilding _array_element_2))
      (:NewEnumerator2
        (CallFunction|GenerateEmptyLot _array_element_2))
      (:NewEnumerator3
        (CallFunction|GenerateCarLot _array_element_2))
      (:NewEnumerator4
        (CallFunction|GeneratePark _array_element_2)))))

(fn GenerateProps)

(fn GenerateCarLot
  (params (Transform :type Transform))
  (for _index (range 1 9)
    (AddComponent|AddStaticMeshComponent false (Math|Transform|MakeTransform (Math|Vector|MakeVector (+ (.x (.location Transform)) (* (LocalVariables|GetCarSpacing) (Math|Conversions|ToFloat(Integer) (- (/ (- _index 1) 3) 1)))) (+ (.y (.location Transform)) (* (LocalVariables|GetCarSpacing) (Math|Conversions|ToFloat(Integer) (- (Math|Integer|%(Integer) _index 3) 1)))) 0.0) "0, 0, 0" (.scale Transform)))))

(fn GeneratePark
  (params (Transform :type Transform))
  (for _index (range 3 (Math|Random|RandomIntegerinRange 4 10))
    (AddComponent|AddStaticMeshComponent false (Math|Transform|MakeTransform (Math|Vector|MakeVector (+ (.x (.location Transform)) (Math|Random|RandomFloatinRange 2e+01 1e+02)) (+ (.y (.location Transform)) (Math|Random|RandomFloatinRange 2e+01 1e+02)) (.z (.location Transform))) (.rotation Transform) (.scale Transform))))
  (for _index_2 (range 3 (Math|Random|RandomIntegerinRange 4 10))
    (AddComponent|AddStaticMeshComponent false (Math|Transform|MakeTransform (Math|Vector|MakeVector (+ (.x (.location Transform)) (Math|Random|RandomFloatinRange 2e+01 1e+02)) (+ (.y (.location Transform)) (Math|Random|RandomFloatinRange 2e+01 1e+02)) (.z (.location Transform))) (.rotation Transform) (.scale Transform)))))

(fn RandomizeLotType
  (bind _output_get (LocalVariables|SetLotSeed (Math|Random|RandomIntegerinRange 0 100)))
  (if (Utilities|InRange? 0 65 _output_get)
    (return "NewEnumerator0")
    (elif (Utilities|InRange? 66 75 _output_get)
      (return "NewEnumerator1")
      (elif (Utilities|InRange? 76 85 _output_get)
        (return "NewEnumerator2")
        (elif (Utilities|InRange? 86 90 _output_get)
          (return "NewEnumerator3")
          (elif (Utilities|InRange? 91 100 _output_get)
            (return "NewEnumerator4")))))))

(fn GenerateApartment
  (params (Transform :type Transform))
  (AddComponent|AddChildActorComponent false Transform))

(fn GenerateSpecialBuilding
  (params (Transform :type Transform))
  (switch int (Math|Random|RandomIntegerinRange 0 8)
    (:0
      (AddComponent|AddStaticMeshComponent false Transform))
    (:1
      (AddComponent|AddStaticMeshComponent false Transform))
    (:2
      (AddComponent|AddStaticMeshComponent false Transform))
    (:3
      (AddComponent|AddStaticMeshComponent false Transform))
    (:4
      (AddComponent|AddStaticMeshComponent false Transform))
    (:5
      (AddComponent|AddStaticMeshComponent false Transform))
    (:6
      (AddComponent|AddStaticMeshComponent false Transform))
    (:7
      (AddComponent|AddStaticMeshComponent false Transform))))

(fn GenerateEmptyLot
  (params (Transform :type Transform))
  (bind _returnvalue (Math|Random|RandomUnitVector))
  (bind _spread (LocalVariables|GetSpread))
  (for _index (range 0 (Math|Random|RandomIntegerinRange 0 10))
    (AddComponent|AddStaticMeshComponent false (Math|Transform|MakeTransform (Math|Vector|MakeVector (+ (.x (.location Transform)) (* (.x _returnvalue) _spread)) (+ (.y (.location Transform)) (* (.y _returnvalue) _spread)) (.z (.location Transform))) (Math|Rotator|MakeRotator 0.0 0.0 (Math|Random|RandomFloatinRange 0.0 3.6e+02)) (.scale Transform)))))