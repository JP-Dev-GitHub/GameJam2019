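; Test actor that procedurally spawns a randomly sized building out of ChunkClassReference actors.
; After a short delay, BeginPlay rolls width, length and floor count, then counts down width × length × floors, spawning a chunk each step.
; Modulo and division on the index give grid offsets, using a perimeter-based chunks-per-floor figure that differs from the full-volume total.
; Debug drawing, printing and a construction-script preview are disconnected.
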(event EventBeginPlay
  (bind _blocksize (Variables|ProceduralParameters|GetBlockSize))
  (Utilities|FlowControl|Delay 0.2)
  (Variables|ProceduralParameters|SetWidthInChunks (Math|Random|RandomIntegerinRange 1 _blocksize))
  (Variables|ProceduralParameters|SetLengthInChunks (Math|Random|RandomIntegerinRange 1 _blocksize))
  (Variables|ProceduralParameters|SetHeightInFloors (Math|Random|RandomIntegerinRange 1 20))
  (Variables|Default|SetTotalChunks (* (* (Variables|ProceduralParameters|GetHeightInFloors) (Variables|ProceduralParameters|GetWidthInChunks)) (Variables|ProceduralParameters|GetLengthInChunks)))
  (while (> (Variables|Default|GetTotalChunks) 0)
    (Math|Integer|DecrementInt (Variables|Default|GetTotalChunks)
      (:%20%20
        (Game|SpawnActorfromClass (Variables|ProceduralParameters|GetChunkClassReference) (Math|Transform|MakeTransform (+ (Math|Vector|MakeVector (* (/ (Math|Integer|%(Integer) (+ (Variables|Default|GetTotalChunks) 1) (+ (* (Variables|ProceduralParameters|GetLengthInChunks) 2) (* (- (Variables|ProceduralParameters|GetWidthInChunks) 2) 2))) (Variables|ProceduralParameters|GetWidthInChunks)) (Variables|Default|GetChunkScale)) (* (Math|Integer|%(Integer) (Math|Integer|%(Integer) (+ (Variables|Default|GetTotalChunks) 1) (+ (* (Variables|ProceduralParameters|GetLengthInChunks) 2) (* (- (Variables|ProceduralParameters|GetWidthInChunks) 2) 2))) (Variables|ProceduralParameters|GetWidthInChunks)) (Variables|Default|GetChunkScale)) (* (/ (Variables|Default|GetTotalChunks) (+ (* (Variables|ProceduralParameters|GetLengthInChunks) 2) (* (- (Variables|ProceduralParameters|GetWidthInChunks) 2) 2))) (Variables|Default|GetChunkScale))) (Transformation|GetWorldLocation (Variables|Default|GetDefaultSceneRoot self))) "0, 0, 0" "1,1,1") "Undefined" 0 0)))))

(event Collision|EventActorBeginOverlap
  (params (OtherActor :type Actor%20Object%20Reference)))

(event EventTick
  (params (DeltaSeconds :type Float%20%28single-precision%29)))

(fn ConstructionScript)