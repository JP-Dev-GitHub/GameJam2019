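; VR mech arm actor that mirrors one motion controller and attaches a cable to the matching mech shoulder.
; Setup snaps it to a hand-relative offset, then Tick projects an anchor from the mech shoulder along the player's shoulder-to-hand direction, scaled by camera-to-hand distance.
; Location and rotation interpolate toward that anchor and controller rotation at a speed-based sync rate, which drops to minimum above the speed limit.
; Debug sphere and prints remain active.
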(event Custom|MechArmSetup
  (CallFunction|HandleLeftHand)
  (bind _returnvalue (CallFunction|CalculateOffset))
  (bind _output_get (Variables|Default|SetAnchorLocation _returnvalue))
  (Transformation|SetActorLocation _output_get false false)
  (bind _output_get_2 (Variables|Default|SetParentHandRotation (Transformation|GetWorldRotation (Variables|/Game/VirtualRealityBP/Blueprints/BP_MotionController.BP_MotionController_C|GetMotionController (Variables|Default|GetParentHand)))))
  (Transformation|SetActorRotation _output_get_2)
  (Variables|Default|SetActive? true))

(event EventTick
  (params (DeltaSeconds :type Float%20%28single-precision%29))
  (bind _returnvalue (Utilities|Time|GetWorldDeltaSeconds))
  (if (Variables|Default|GetActive?)
    (Utilities|IsValid (Variables|Default|GetParentHand)
      (:Is%20Valid
        (Utilities|FlowControl|Sequence
          (:then_0
            (bind _offset (CallFunction|TestOffset))
            (bind _output_get (Variables|Default|SetAnchorLocation _offset))
            (Variables|Default|SetParentHandRotation (Transformation|GetWorldRotation (Variables|/Game/VirtualRealityBP/Blueprints/BP_MotionController.BP_MotionController_C|GetMotionController (Variables|Default|GetParentHand))))
            (Variables|Default|SetFramesWaited 0)
            (Rendering|Debug|DrawDebugSphere _output_get 11.0 22 "(R=0.224927,G=1.000000,B=0.000000,A=1.000000)" 0.0 0.7))
          (:then_1
            (bind _newsyncrate (CallFunction|CalculateSyncRate))
            (Variables|Default|SetSyncRate _newsyncrate))
          (:then_2
            (Transformation|SetActorLocationAndRotation (Math|Interpolation|VInterpTo (Transformation|GetActorLocation) (Variables|Default|GetAnchorLocation) _returnvalue (Variables|Default|GetSyncRate)) (Math|Interpolation|RInterpTo (Transformation|GetActorRotation) (Variables|Default|GetParentHandRotation) _returnvalue (Variables|Default|GetSyncRate))))
          (:then_3
            (Development|PrintString (Utilities|String|Append "Sync Rate: " (Utilities|String|ToString(Float) (Variables|Default|GetSyncRate))) true true "(R=0.174191,G=1.000000,B=0.000000,A=1.000000)" 0.0)))))))

(fn ConstructionScript)

(fn HandleLeftHand
  (bind _parenthand (Variables|Default|GetParentHand))
  (bind _playerref (Variables|/Game/VirtualRealityBP/Blueprints/BP_MotionController.BP_MotionController_C|GetPlayerRef _parenthand))
  (switch Utilities|FlowControl|Switch|SwitchonEControllerHand (Variables|Default|GetHand)
    (:Left
      (Transformation|SetRelativeRotation (Variables|Default|GetMeshRoot) "0, 0, 0" false false)
      (Class|CableComponent|SetAttachEndtoComponent (Variables|Default|GetCable) (Variables|/Game/ArmIK/MechPawn.MechPawn_C|GetMechShoulder_L _playerref) "None"))
    (:Right
      (Class|CableComponent|SetAttachEndtoComponent (Variables|Default|GetCable) (Variables|/Game/ArmIK/MechPawn.MechPawn_C|GetMechShoulder_R _playerref) "None"))))

(fn CalculateSyncRate
  (bind _parenthand (Variables|Default|GetParentHand))
  (bind _controllerspeed (Variables|/Game/VirtualRealityBP/Blueprints/BP_MotionController.BP_MotionController_C|GetControllerSpeed _parenthand))
  (if (Math|Float|InRange(Float) _controllerspeed -1.0 (Variables|Default|GetHandSpeedLimit))
    (return (Math|Float|Lerp (Variables|Default|GetMinSyncRate) (Variables|Default|GetMaxSyncRate) (/ _controllerspeed (Variables|Default|GetHandSpeedLimit))))
    (else
      (return (Variables|Default|GetMinSyncRate)))))

(fn CalculateTargetLocation
  (bind _parenthand (Variables|Default|GetParentHand))
  (bind _parenthand_2 (Variables|Default|GetParentHand))
  (bind _distscalar (LocalVariables|GetDistScalar))
  (bind _armoffset (Variables|Default|GetArmOffset))
  (bind _distscalar_2 (LocalVariables|GetDistScalar))
  (if (Utilities|Enum|Equal(Enum) (Variables|Default|GetHand) "Left")
    (return (+ (Variables|Default|GetAnchorLocation) (* (Transformation|GetActorForwardVector _parenthand) (* (.x _distscalar) 0.0)) (* (Math|Vector|GetRightVector (Variables|/Game/ArmIK/MechPawn.MechPawn_C|GetCamera (Variables|/Game/VirtualRealityBP/Blueprints/BP_MotionController.BP_MotionController_C|GetPlayerRef (Variables|Default|GetParentHand)))) (* (* (.y _distscalar) 0.0) -1.0)) (* (Transformation|GetActorUpVector _parenthand) (* (.z _distscalar) 0.0))))
    (else
      (return (+ (Variables|Default|GetAnchorLocation) (* (Transformation|GetActorForwardVector _parenthand_2) (* (.x _distscalar_2) (.x _armoffset))) (* (Math|Vector|GetRightVector (Variables|/Game/ArmIK/MechPawn.MechPawn_C|GetCamera (Variables|/Game/VirtualRealityBP/Blueprints/BP_MotionController.BP_MotionController_C|GetPlayerRef (Variables|Default|GetParentHand)))) (* (.y _distscalar_2) (.y _armoffset))) (* (Transformation|GetActorUpVector _parenthand_2) (* (.z _distscalar_2) (.z _armoffset))))))))

(fn CalculateDistanceScalar
  (bind _parenthand (Variables|Default|GetParentHand))
  (bind _playerref (Variables|/Game/VirtualRealityBP/Blueprints/BP_MotionController.BP_MotionController_C|GetPlayerRef _parenthand))
  (bind _camera (Variables|/Game/ArmIK/MechPawn.MechPawn_C|GetCamera _playerref))
  (return (Math|Float|Clamp(Float) (/ (Math|Vector|VectorLength (- (Transformation|GetWorldLocation (Variables|/Game/VirtualRealityBP/Blueprints/BP_MotionController.BP_MotionController_C|GetMotionController _parenthand)) (+ (Transformation|GetWorldLocation _camera) (* (Math|Vector|GetUpVector _camera) -2e+01)))) 7e+01))))

(fn CalculateOffset
  (bind _scalar (CallFunction|CalculateDistanceScalar))
  (bind _scalar_2 (CallFunction|CalculateDistanceScalar))
  (bind _minmaxdown (Variables|Default|GetMinMaxDown))
  (bind _minmaxforward (Variables|Default|GetMinMaxForward))
  (bind _minmaxright (Variables|Default|GetMinMaxRight))
  (bind _minmaxforward_2 (Variables|Default|GetMinMaxForward))
  (bind _minmaxdown_2 (Variables|Default|GetMinMaxDown))
  (bind _parenthand (Variables|Default|GetParentHand))
  (bind _parenthand_2 (Variables|Default|GetParentHand))
  (bind _minmaxright_2 (Variables|Default|GetMinMaxRight))
  (bind _motioncontroller (Variables|/Game/VirtualRealityBP/Blueprints/BP_MotionController.BP_MotionController_C|GetMotionController _parenthand))
  (bind _motioncontroller_2 (Variables|/Game/VirtualRealityBP/Blueprints/BP_MotionController.BP_MotionController_C|GetMotionController _parenthand_2))
  (Development|PrintString (Utilities|String|Append "Dist Scalar: " (Utilities|String|ToString(Float) (CallFunction|CalculateDistanceScalar))) true true "(R=1.000000,G=0.000000,B=0.059606,A=1.000000)" 0.0)
  (if (Utilities|Enum|Equal(Enum) (Variables|Default|GetHand) "Right")
    (return (+ (Transformation|GetWorldLocation _motioncontroller) (* (Math|Vector|GetForwardVector _motioncontroller) (Math|Float|Lerp (.x _minmaxforward_2) (.y _minmaxforward_2) _scalar_2)) (* (Math|Vector|GetUpVector _motioncontroller) (Math|Float|Lerp (.x _minmaxdown_2) (.y _minmaxdown_2) _scalar_2)) (* (Math|Vector|GetRightVector (Variables|/Game/ArmIK/MechPawn.MechPawn_C|GetCamera (Variables|/Game/VirtualRealityBP/Blueprints/BP_MotionController.BP_MotionController_C|GetPlayerRef (Variables|Default|GetParentHand)))) (Math|Float|Lerp (.x _minmaxright) (.y _minmaxright) _scalar_2))))
    (else
      (return (+ (Transformation|GetWorldLocation _motioncontroller_2) (* (Math|Vector|GetForwardVector _motioncontroller_2) (Math|Float|Lerp (.x _minmaxforward) (.y _minmaxforward) _scalar)) (* (Math|Vector|GetUpVector _motioncontroller_2) (Math|Float|Lerp (.x _minmaxdown) (.y _minmaxdown) _scalar)) (* (Math|Vector|GetRightVector (Variables|/Game/ArmIK/MechPawn.MechPawn_C|GetCamera (Variables|/Game/VirtualRealityBP/Blueprints/BP_MotionController.BP_MotionController_C|GetPlayerRef _parenthand_2))) (Math|Float|Lerp (* (.x _minmaxright_2) -1.0) (* (.y _minmaxright_2) -1.0) _scalar)))))))

(fn TestOffset
  (bind _parenthand (Variables|Default|GetParentHand))
  (bind _parenthand_2 (Variables|Default|GetParentHand))
  (if (Utilities|Enum|Equal(Enum) (Variables|Default|GetHand) "Right")
    (LocalVariables|SetRightDirection (Math|Vector|Normalize (- (Transformation|GetWorldLocation (Variables|/Game/VirtualRealityBP/Blueprints/BP_MotionController.BP_MotionController_C|GetMotionController _parenthand_2)) (Transformation|GetWorldLocation (Variables|/Game/ArmIK/MechPawn.MechPawn_C|GetPlayerShoulder_R (Variables|/Game/VirtualRealityBP/Blueprints/BP_MotionController.BP_MotionController_C|GetPlayerRef _parenthand_2))))))
    (return (+ (Transformation|GetWorldLocation (Variables|/Game/ArmIK/MechPawn.MechPawn_C|GetMechShoulder_R (Variables|/Game/VirtualRealityBP/Blueprints/BP_MotionController.BP_MotionController_C|GetPlayerRef (Variables|Default|GetParentHand)))) (* (LocalVariables|GetRightDirection) (Math|Float|Lerp 4e+02 7.5e+02 (CallFunction|CalculateDistanceScalar)))))
    (else
      (LocalVariables|SetRightDirection (Math|Vector|Normalize (- (Transformation|GetWorldLocation (Variables|/Game/VirtualRealityBP/Blueprints/BP_MotionController.BP_MotionController_C|GetMotionController _parenthand)) (Transformation|GetWorldLocation (Variables|/Game/ArmIK/MechPawn.MechPawn_C|GetPlayerShoulder_L (Variables|/Game/VirtualRealityBP/Blueprints/BP_MotionController.BP_MotionController_C|GetPlayerRef _parenthand))))))
      (return (+ (Transformation|GetWorldLocation (Variables|/Game/ArmIK/MechPawn.MechPawn_C|GetMechShoulder_L (Variables|/Game/VirtualRealityBP/Blueprints/BP_MotionController.BP_MotionController_C|GetPlayerRef (Variables|Default|GetParentHand)))) (* (LocalVariables|GetRightDirection) (Math|Float|Lerp 4e+02 7.5e+02 (CallFunction|CalculateDistanceScalar))))))))