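; Twin-barrel weapon actor that, despite its missile launcher name, fires colored LaserBolt_BP projectiles alternately from left and right spawn points.
; FireLauncher is rate-limited by CanFire and a reset timer, and a FlipFlop picks the side for each bolt, sound and particle burst.
; The same FlipFlop drives a per-side timeline that animates that launcher mesh along X.
; The construction script applies Color to both spawn particles.
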(event Custom|FireLauncher
  (bind _launchermesh_l (Variables|Default|GetLauncherMesh_L))
  (bind _launchermesh_r (Variables|Default|GetLauncherMesh_R))
  (bind _projectilespawnpoint_l (Variables|Default|GetProjectileSpawnPoint_L))
  (bind _projectilespawnpoint_r (Variables|Default|GetProjectileSpawnPoint_R))
  (bind _returnvalue (Transformation|GetWorldTransform _projectilespawnpoint_r))
  (bind _returnvalue_2 (Transformation|GetWorldTransform _projectilespawnpoint_l))
  (bind _relativelocation (Variables|/Script/Engine.SceneComponent|GetRelativeLocation _launchermesh_r))
  (bind _relativelocation_2 (Variables|/Script/Engine.SceneComponent|GetRelativeLocation _launchermesh_l))
  (if (Variables|Default|GetCanFire?)
    (Variables|Default|SetCanFire? false)
    (Utilities|Time|SetTimerbyFunctionName 0 "ResetCanFire" (Variables|Default|GetFireRateDelay))
    (Utilities|FlowControl|Sequence
      (:then_0
        (bind _isa (Utilities|FlowControl|FlipFlop)
          (:A
            (bind _returnvalue_3 (Game|SpawnActorfromClass "/Game/AI/Enemies/EnemyBPs/LaserBolt_BP.LaserBolt_BP_C" (Math|Transform|MakeTransform (.location _returnvalue_2) (Math|Rotator|FindLookatRotation (.location _returnvalue_2) (+ (.location _returnvalue_2) (* (Math|Vector|GetForwardVector _projectilespawnpoint_l) 1.2e+03))) (.scale _returnvalue_2)) "Undefined" 0 50 true 0 "NewEnumerator0" 0))
            (Default|SetParticleColor _returnvalue_3 (Variables|Default|GetColor))
            (Components|Activation|Activate (Variables|Default|GetFireSFX_L) true))
          (:B
            (bind _returnvalue_4 (Game|SpawnActorfromClass "/Game/AI/Enemies/EnemyBPs/LaserBolt_BP.LaserBolt_BP_C" (Math|Transform|MakeTransform (.location _returnvalue) (Math|Rotator|FindLookatRotation (.location _returnvalue) (+ (.location _returnvalue) (* (Math|Vector|GetForwardVector _projectilespawnpoint_r) 1.2e+03))) (.scale _returnvalue)) "Undefined" 0 50 true 0 "NewEnumerator0" 0))
            (Default|SetParticleColor _returnvalue_4 (Variables|Default|GetColor))
            (Components|Activation|Activate (Variables|Default|GetFireSFX_R) true))))
      (:then_1
        (if _isa
          (bind _alpha (Timeline|LeftFire PlayFromStart)
            (:Update
              (Transformation|SetRelativeLocation _launchermesh_l (Math|Vector|MakeVector _alpha (.y _relativelocation_2) (.z _relativelocation_2)) false false)))
          (else
            (bind _alpha_2 (Timeline|RightFire PlayFromStart)
              (:Update
                (Transformation|SetRelativeLocation _launchermesh_r (Math|Vector|MakeVector _alpha_2 (.y _relativelocation) (.z _relativelocation)) false false)))))))))

(event EventBeginPlay)

(fn ConstructionScript
  (Effects|Components|ParticleSystem|SetVectorParameter (Variables|Default|GetSpawnParticle_R) "Color" (Math|Conversions|ToVector(LinearColor) (Variables|Default|GetColor))))

(fn ResetCanFire
  (Variables|Default|SetCanFire? true))