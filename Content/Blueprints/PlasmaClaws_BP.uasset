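; Plasma claw weapon that toggles on and off and slices procedural meshes when swung fast enough, apparently in VR.
; ToggleSaber scales the claw mesh along X via a timeline, with ignite and retract sounds.
; Blade planes spark on overlap; blade 1, when active, slices on exit, messaging the hit actor or re-slicing "Sliced" pieces itself into physics halves.
; Blade 2's slicing is disconnected, and its sparks ignore the active state.
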(event OnComponentBeginOverlap(ProceduralPlane01)
  (params (OverlappedComponent :type Primitive%20Component%20Object%20Reference) (OtherActor :type Actor%20Object%20Reference) (OtherComp :type Primitive%20Component%20Object%20Reference) (OtherBodyIndex :type Integer) (bFromSweep :type Boolean) (SweepResult :type Hit%20Result%20Structure%20%28by%20ref%29))
  (bind _proceduralplane01 (Variables|Default|GetProceduralPlane01))
  ;[1 1 1] Blade 1 Slice
  (bind _asprocedural_mesh_component (Utilities|Casting|CastToProceduralMeshComponent OtherComp))
  (if (and (Variables|Default|GetActive?) (Utilities|Enum|Equal(Enum) (Collision|GetCollisionObjectType OtherComp) "ECC_GameTraceChannel6"))
    (bind _mincutspeed (Class|SliceableInterface|GetMinSliceSpeed(Message) _asprocedural_mesh_component))
    (bind _speed (CallFunction|GetSlicerSpeed))
    (if (> _speed _mincutspeed)
      (bind _returnvalue (Effects|SpawnEmitteratLocation "/Game/Particles/P_SliceSparks.P_SliceSparks" (Transformation|GetWorldLocation _proceduralplane01) (Transformation|GetWorldRotation _proceduralplane01)))
      (Effects|Components|ParticleSystem|SetVectorParameter _returnvalue "Color" (Math|Conversions|ToVector(LinearColor) (Variables|Default|GetBladeColor))))))

(event OnComponentEndOverlap(ProceduralPlane01)
  (params (OverlappedComponent :type Primitive%20Component%20Object%20Reference) (OtherActor :type Actor%20Object%20Reference) (OtherComp :type Primitive%20Component%20Object%20Reference) (OtherBodyIndex :type Integer))
  ;[1 1 1] Blade 1 Slice
  (bind _asprocedural_mesh_component (Utilities|Casting|CastToProceduralMeshComponent OtherComp))
  (if (and (Variables|Default|GetActive?) (Utilities|Enum|Equal(Enum) (Collision|GetCollisionObjectType OtherComp) "ECC_GameTraceChannel6"))
    (bind _mincutspeed (Class|SliceableInterface|GetMinSliceSpeed(Message) _asprocedural_mesh_component))
    (bind _speed (CallFunction|GetSlicerSpeed))
    (if (> _speed _mincutspeed)
      (bind _slice (CallFunction|GetSliceInfo (Variables|Default|GetProceduralPlane01)))
      (if (Components|ComponentHasTag OtherComp "Sliced")
        (CallFunction|SliceRogueMesh _asprocedural_mesh_component _slice)
        (else
          (Class|SliceableInterface|SliceMesh(Message) OtherActor (Variables|Default|GetProceduralPlane01) _asprocedural_mesh_component _slice))))))

(event OnComponentBeginOverlap(ProceduralPlane02)
  (params (OverlappedComponent :type Primitive%20Component%20Object%20Reference) (OtherActor :type Actor%20Object%20Reference) (OtherComp :type Primitive%20Component%20Object%20Reference) (OtherBodyIndex :type Integer) (bFromSweep :type Boolean) (SweepResult :type Hit%20Result%20Structure%20%28by%20ref%29))
  (bind _proceduralplane02 (Variables|Default|GetProceduralPlane02))
  ;[1 1 1] Blade 2 Slice
  (bind _asprocedural_mesh_component (Utilities|Casting|CastToProceduralMeshComponent OtherComp))
  (if (Utilities|Enum|Equal(Enum) (Collision|GetCollisionObjectType OtherComp) "ECC_GameTraceChannel6")
    (bind _mincutspeed (Class|SliceableInterface|GetMinSliceSpeed(Message) _asprocedural_mesh_component))
    (bind _speed (CallFunction|GetSlicerSpeed))
    (if (> _speed _mincutspeed)
      (bind _returnvalue (Effects|SpawnEmitteratLocation "/Game/Particles/P_SliceSparks.P_SliceSparks" (Transformation|GetWorldLocation _proceduralplane02) (Transformation|GetWorldRotation _proceduralplane02)))
      (Effects|Components|ParticleSystem|SetVectorParameter _returnvalue "Color" (Math|Conversions|ToVector(LinearColor) (Variables|Default|GetBladeColor))))))

(event OnComponentEndOverlap(ProceduralPlane02)
  (params (OverlappedComponent :type Primitive%20Component%20Object%20Reference) (OtherActor :type Actor%20Object%20Reference) (OtherComp :type Primitive%20Component%20Object%20Reference) (OtherBodyIndex :type Integer))
  ;[1 1 1] Blade 2 Slice
)

(event Custom|ToggleSaber
  (bind _returnvalue (Transformation|GetActorLocation))
  (Utilities|FlowControl|FlipFlop
    (:A
      (Variables|Default|SetActive? true)
      (Audio|PlaySoundatLocation "/Game/Audio/plasmaIgnite_Cue.PlasmaIgnite_Cue" _returnvalue "0, 0, 0" 1.0 1.0 0.0 0 0 0)
      (Rendering|SetVisibility (Variables|Default|GetClawMesh) true false)
      (bind _alpha (Timeline|Saber_TL PlayFromStart)
        (:Update
          (Transformation|SetRelativeScale3D (Variables|Default|GetClawMesh) (Math|Vector|Lerp(Vector) (Variables|Default|GetOffScale) (Variables|Default|GetOG_RelativeScale) _alpha)))
        (:Finished
          (Rendering|SetVisibility (Variables|Default|GetClawMesh) (Variables|Default|GetActive?) false))))
    (:B
      (Variables|Default|SetActive? false)
      (Audio|PlaySoundatLocation "/Game/Audio/plasmaRetract_Cue.PlasmaRetract_Cue" _returnvalue "0, 0, 0" 1.0 1.0 0.0 0 0 0)
      (Timeline|Saber_TL ReverseFromEnd))))

(event EventBeginPlay
  (bind _output_get (Variables|Default|SetOG_RelativeScale (Variables|/Script/Engine.SceneComponent|GetRelativeScale3D (Variables|Default|GetClawMesh))))
  (bind _output_get_2 (Variables|Default|SetOffScale (Math|Vector|MakeVector 0.0 (.Y (Math|Vector|BreakVector _output_get)) (.Z (Math|Vector|BreakVector _output_get)))))
  (Transformation|SetRelativeScale3D (Variables|Default|GetClawMesh) _output_get_2)
  (Rendering|SetVisibility (Variables|Default|GetClawMesh) (Variables|Default|GetActive?) false))

(fn ConstructionScript
  (Rendering|Material|SetVectorParameterValueonMaterials (Variables|Default|GetClawMesh) "Color" (Math|Conversions|ToVector(LinearColor) (Variables|Default|GetBladeColor))))

(fn SliceRogueMesh
  (params (Component :type Procedural%20Mesh%20Component%20Object%20Reference) (SliceInfo :type Slice%20Info%20Structure))
  (Utilities|FlowControl|Sequence
    (:then_0
      (bind _returnvalue (Effects|SpawnEmitteratLocation "/Game/Particles/P_SliceSparks.P_SliceSparks" (.sliceposition SliceInfo)))
      (Effects|Components|ParticleSystem|SetVectorParameter _returnvalue "Color" (Math|Conversions|ToVector(LinearColor) (Variables|Default|GetBladeColor))))
    (:then_1
      (bind _outotherhalfprocmesh (Class|KismetProceduralMeshLibrary|SliceProceduralMesh Component (.sliceposition SliceInfo) (.slicenormal SliceInfo) (.createotherhalf? SliceInfo) "CreateNewSectionForCap" (.slicematerial SliceInfo)))
      (Utilities|FlowControl|Sequence
        (:then_0
          (Collision|SetCollisionObjectType _outotherhalfprocmesh "ECC_GameTraceChannel6")
          (Collision|SetCollisionResponsetoAllChannels _outotherhalfprocmesh "ECR_Block")
          (Collision|SetCollisionEnabled _outotherhalfprocmesh "QueryAndPhysics")
          (Physics|SetSimulatePhysics _outotherhalfprocmesh true)
          (Physics|SetEnableGravity _outotherhalfprocmesh true)
          (Physics|AddRadialImpulse _outotherhalfprocmesh (.sliceposition SliceInfo) 3e+02 6e+02 "RIF_Constant" true)
          (Variables|/Script/Engine.ActorComponent|SetComponentTags _outotherhalfprocmesh (Utilities|Array|MakeArray "Sliced")))
        (:then_1
          (Development|PrintString (Utilities|GetDisplayName (Components|GetOwner Component))))))))

(fn GetSliceInfo
  (params (SliceComponent :type Scene%20Component%20Object%20Reference))
  (bind _proceduralplane01 (Variables|Default|GetProceduralPlane01))
  (bind _proceduralplane02 (Variables|Default|GetProceduralPlane02))
  (if (== SliceComponent _proceduralplane01)
    (return (Utilities|Struct|MakeSliceInfo (Transformation|GetWorldLocation _proceduralplane01) (Math|Vector|GetUpVector _proceduralplane01) true "/Game/Materials/M_Plastic_Inst.M_Plastic_Inst"))
    (elif (== SliceComponent _proceduralplane02)
      (return (Utilities|Struct|MakeSliceInfo (Transformation|GetWorldLocation _proceduralplane02) (Math|Vector|GetUpVector _proceduralplane02) true "/Game/Materials/M_Plastic_Inst.M_Plastic_Inst"))
      (else
        (return "")))))

(fn GetSlicerSpeed
  (bind _hand (Variables|Default|GetHand))
  (if (Utilities|Enum|Equal(Enum) _hand "AnyHand")
    (return 9999999.0)
    (else
      (return (CallFunction|GetControllerSpeed _hand)))))