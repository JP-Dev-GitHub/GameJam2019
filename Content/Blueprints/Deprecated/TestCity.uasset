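; TestCity is a deprecated test actor that builds a square city of procedural buildings when play begins.
; It spawns a ProceduralBuildingTemplate at its own transform for each block in a CitySizeInBlocks-sided grid.
; After each spawn it teleports itself to the next cell row by row, acting as the placement cursor.
; Cell spacing comes from the spawned building's block size times chunk scale, offset from the actor's initial location.
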(event EventBeginPlay
  (Variables|Default|SetInitialLocation (Transformation|GetActorLocation self))
  (Variables|Default|SetTotalBlocks (* (Variables|Parameters|GetCitySizeInBlocks) (Variables|Parameters|GetCitySizeInBlocks)))
  (while (> (Variables|Default|GetTotalBlocks) 0)
    (bind _returnvalue (Game|SpawnActorfromClass (Variables|Parameters|GetProceduralBuildingTemplate) (Transformation|GetActorTransform self) "Undefined" 0 0))
    (Variables|Default|SetStepSize (* (Variables|/Game/Blueprints/Deprecated/TestBuilding.TestBuilding_C|GetBlockSize _returnvalue) (Variables|/Game/Blueprints/Deprecated/TestBuilding.TestBuilding_C|GetChunkScale _returnvalue)))
    (Math|Integer|DecrementInt (Variables|Default|GetTotalBlocks)
      (:%20%20
        (if (== (Variables|Default|GetStepsTaken) (- (Variables|Parameters|GetCitySizeInBlocks) 1))
          (Variables|Default|SetStepsTaken 0)
          (Math|Integer|IncrementInt (Variables|Default|GetRowsCompleted)
            (:%20%20
              _))
          (else
            (Math|Integer|IncrementInt (Variables|Default|GetStepsTaken)
              (:%20%20
                _))))
        (Transformation|SetActorLocation (+ (Math|Vector|MakeVector (* (Variables|Default|GetStepsTaken) (Variables|Default|GetStepSize)) (* (Variables|Default|GetRowsCompleted) (Variables|Default|GetStepSize)) 0.0) (Variables|Default|GetInitialLocation)) false false)))))

(fn ConstructionScript)