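; Deprecated VR climbable cube, made for an older MotionControllerPawn, that lets the player climb by gripping it with motion controllers.
; Climb and Release track up to two gripping hands, keep the pawn's ClimbingHands count and re-anchor PivotPoint to the active hand, favoring the second.
; While climbing, Tick offsets the pawn by the active hand's drift from the pivot, without sweep, then pins that controller back on the pivot.
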(event EventTick
  (params (DeltaSeconds :type Float%20%28single-precision%29))
  (bind _firstmotioncontroller (Variables|Default|GetFirstMotionController))
  (bind _secondmotioncontroller (Variables|Default|GetSecondMotionController))
  (bind _secondmotioncontroller_2 (Variables|Default|GetSecondMotionController))
  (bind _returnvalue (Utilities|IsValid _secondmotioncontroller))
  (bind _returnvalue_2 (select _returnvalue _secondmotioncontroller_2 _firstmotioncontroller))
  (if (Utilities|IsValid (Variables|Default|GetMotionControllerPawn))
    (if (and (Variables|/Game/VirtualRealityBP/Blueprints/MotionControllerPawn.MotionControllerPawn_C|GetIsClimbing (Variables|Default|GetMotionControllerPawn)) (Utilities|IsValid (Variables|Default|GetFirstMotionController)))
      (Transformation|AddActorWorldOffset (Variables|Default|GetMotionControllerPawn) (- (Variables|Default|GetPivotPoint) (Transformation|GetWorldLocation _returnvalue_2)))
      (Transformation|SetWorldLocation _returnvalue_2 (Variables|Default|GetPivotPoint) false false) ; Neutralize hand movement due to pawn motion
    )))

(event EventClimb
  (params (MotionController :type Scene%20Component%20Object%20Reference))
  ;[1 1 1] Set the motion controller to the appropriate holding reference
  (if (Utilities|IsValid (Variables|Default|GetFirstMotionController))
    (Variables|Default|SetSecondMotionController MotionController)
    (else
      (Variables|Default|SetFirstMotionController MotionController)))
  ;[1 1 1] Set the pivot to the correct hand, for swinging
  (Variables|Default|SetPivotPoint (Transformation|GetWorldLocation (select (Utilities|IsValid (Variables|Default|GetSecondMotionController)) (Variables|Default|GetSecondMotionController) (Variables|Default|GetFirstMotionController))))
  ;[1 1 1] Increment climbing hands on the pawn
  (bind _asmotion_controller_pawn (Utilities|Casting|CastToMotionControllerPawn (Game|Player|GetPlayerPawn 0)))
  (bind _output_get (Variables|Default|SetMotionControllerPawn _asmotion_controller_pawn))
  (Math|Integer|IncrementInt (Variables|/Game/VirtualRealityBP/Blueprints/MotionControllerPawn.MotionControllerPawn_C|GetClimbingHands _output_get)))

(event EventRelease
  (params (MotionController :type Scene%20Component%20Object%20Reference))
  ;[1 1 1] Determine which hand was released
  (if (Utilities|IsValid (Variables|Default|GetSecondMotionController))
    (if (== (Variables|Default|GetSecondMotionController) MotionController)
      ;[1 1 1] Update Pivot to the appropriate primary hand
      (Variables|Default|SetSecondMotionController 0)
      (Variables|Default|SetPivotPoint (Transformation|GetWorldLocation (Variables|Default|GetFirstMotionController)))
      (else
        (bind _output_get (Variables|Default|SetFirstMotionController (Variables|Default|GetSecondMotionController)))
        (Variables|Default|SetSecondMotionController 0)
        (Variables|Default|SetPivotPoint (Transformation|GetWorldLocation _output_get))))
    ;[1 1 1] Decrement Climbing hands on pawn
    (Utilities|IsValid (Variables|Default|GetMotionControllerPawn) :!label _label
      (:Is%20Valid
        (Math|Integer|DecrementInt (Variables|/Game/VirtualRealityBP/Blueprints/MotionControllerPawn.MotionControllerPawn_C|GetClimbingHands (Variables|Default|GetMotionControllerPawn))))
      (:Is%20Not%20Valid
        (bind _asmotion_controller_pawn (Utilities|Casting|CastToMotionControllerPawn (Game|Player|GetPlayerPawn 0)))
        (bind _output_get_2 (Variables|Default|SetMotionControllerPawn _asmotion_controller_pawn))
        (Math|Integer|DecrementInt (Variables|/Game/VirtualRealityBP/Blueprints/MotionControllerPawn.MotionControllerPawn_C|GetClimbingHands _output_get_2))))
    (elif (== MotionController (Variables|Default|GetFirstMotionController))
      (Variables|Default|SetFirstMotionController 0)
      (Variables|Default|SetSecondMotionController 0)
      (Variables|Default|SetPivotPoint "0, 0, 0")
      (goto _label))))

(fn ConstructionScript)